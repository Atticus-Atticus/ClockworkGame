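; BP_PlatformLonger is a level platform that moves back and forth continuously like an elevator, starting on BeginPlay.
; MoveElevator uses a FlipFlop to alternate the timeline between playing from start and reversing from end, and calls itself again when the timeline finishes.
; Each timeline update lerps the Cube's world location between the BottomPostion and TopPosition components, without sweep.
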(event Custom|MoveElevator
  (Utilities|FlowControl|FlipFlop
    (:A
      (bind _alpha2 (Timeline|Timeline PlayFromStart)
        (:Update
          (Transformation|SetWorldLocation (Variables|Default|GetCube) (Math|Vector|Lerp(Vector) (Transformation|GetWorldLocation (Variables|Default|GetBottomPostion)) (Transformation|GetWorldLocation (Variables|Default|GetTopPosition)) _alpha2) false false))
        (:Finished
          (CallFunction|MoveElevator))))
    (:B
      (Timeline|Timeline ReverseFromEnd))))

(event EventBeginPlay
  (CallFunction|MoveElevator))

(fn ConstructionScript)